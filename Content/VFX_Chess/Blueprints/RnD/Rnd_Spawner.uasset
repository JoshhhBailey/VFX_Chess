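; R&D spawner actor that repeatedly spawns a chess piece character at its own transform.
; Tick feeds a Delay to repeat the spawn at a set interval, with an optional extra spawn on BeginPlay.
; Each spawned Character_BP gets ragdoll enabled, a BoneBreaker destroyed lifespan and walking movement.
; Rook pieces also have their speed overridden.
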(event EventBeginPlay
  (if (Variables|SpawnOptions|GetisSpawnOnBegin)
    (CallFunction|SpawnCharacter)))

(event Collision|EventActorBeginOverlap
  (params (OtherActor :type Actor%20Object%20Reference)))

(event EventTick
  (params (DeltaSeconds :type Float%20%28single-precision%29))
  (Utilities|FlowControl|Delay (Variables|SpawnOptions|GetDelay))
  (CallFunction|SpawnCharacter))

(fn ConstructionScript)

(fn SpawnCharacter
  (bind _returnvalue (Game|SpawnActorfromClass (Variables|SpawnOptions|GetSpawnedPiece) (Transformation|GetActorTransform) "AdjustIfPossibleButAlwaysSpawn" 0 0))
  (bind _ascharacter_bp (Utilities|Casting|CastToCharacter_BP _returnvalue))
  ;[1 1 1] Ragdoll parameters
  (Variables|/Game/VFX_Chess/Blueprints/Character_BP.Character_BP_C|SetRagdollEnabled _ascharacter_bp true)
  (Variables|/Game/VFX_Chess/Blueprints/BoneBreaker.BoneBreaker_C|SetDestroyedLifeSpan (Actor|GetComponentbyClass _ascharacter_bp "/Game/VFX_Chess/Blueprints/BoneBreaker.BoneBreaker_C") (Variables|SpawnOptions|GetSpawnedDestroyedLifeSpan))
  (Pawn|Components|CharacterMovement|SetMovementMode (Variables|/Script/Engine.Character|GetCharacterMovement _ascharacter_bp) "MOVE_Walking" 0)
  (bind _asrook_bp (Utilities|Casting|CastToRook_BP _ascharacter_bp))
  (Variables|/Game/VFX_Chess/Assets/Characters/Rook/Rook_BP.Rook_BP_C|SetRookSpeed _asrook_bp 5e+01))