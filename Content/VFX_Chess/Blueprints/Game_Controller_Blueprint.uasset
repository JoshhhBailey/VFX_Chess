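; Game controller for a chess game that handles sounds, move clocks and UI for captures, promotion, cutscenes and game endings.
; Events play sounds, notify the PlayerHUD of taken pieces, and create promotion, victory, stalemate or cutscene widgets.
; On the main level, SetTimers creates paused per-side timers from the game instance's move time, each awarding the opponent victory on expiry.
; Tick pauses both while the game is paused, otherwise running the moving side's timer after a short delay.
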(event Custom|SetTimers
  ;[1 1 1] Check if the current level is the main level
  (bind _returnvalue (Game|GetCurrentLevelName true))
  (if (Utilities|Enum|Equal(Enum) _returnvalue (Variables|Default|GetMainLevelName))
    ;[1 1 1] Create white and black timers and pause them
    (bind _asvfxgame_instance (Utilities|Casting|CastToVFXGameInstance (Game|GetGameInstance)))
    (Utilities|FlowControl|Sequence
      (:then_0
        (bind _returnvalue_2 (Utilities|Time|SetTimerbyEvent (delegate EventBlackWin) (Variables|/Game/VFX_Chess/Blueprints/VFXGameInstance.VFXGameInstance_C|GetTimeToMove _asvfxgame_instance)))
        (bind _output_get (Variables|Default|SetWhiteTimer _returnvalue_2))
        (Utilities|Time|PauseTimerbyHandle _output_get))
      (:then_1
        (bind _returnvalue_3 (Utilities|Time|SetTimerbyEvent (delegate EventWhiteWin) (Variables|/Game/VFX_Chess/Blueprints/VFXGameInstance.VFXGameInstance_C|GetTimeToMove _asvfxgame_instance)))
        (bind _output_get_2 (Variables|Default|SetBlackTimer _returnvalue_3))
        (Utilities|Time|PauseTimerbyHandle _output_get_2)))
    (Variables|Default|SetTimersSet true)))

(event EventBeginPlay)

(event EventTick
  (params (DeltaSeconds :type Float%20%28single-precision%29))
  ;[1 1 1] Pause timers if the game is paused
  (if (Game|IsGamePaused)
    (Utilities|FlowControl|Sequence
      (:then_0
        (Utilities|Time|PauseTimerbyHandle (Variables|Default|GetWhiteTimer)))
      (:then_1
        (Utilities|Time|PauseTimerbyHandle (Variables|Default|GetBlackTimer))))
    (else
      ;[1 1 1] Check which pieces move and pause/unpause the timers accordingly
      (bind _returnvalue (Class|GameController|GetWhiteMove))
      (if _returnvalue
        (Utilities|Time|PauseTimerbyHandle (Variables|Default|GetBlackTimer))
        (Utilities|FlowControl|Delay 2.0)
        (Utilities|Time|UnpauseTimerbyHandle (Variables|Default|GetWhiteTimer))
        (else
          (Utilities|Time|PauseTimerbyHandle (Variables|Default|GetWhiteTimer))
          (Utilities|FlowControl|Delay 2.0)
          (Utilities|Time|UnpauseTimerbyHandle (Variables|Default|GetBlackTimer)))))))

(event EventCallCutscene
  (params (_index :type Integer))
  (bind _returnvalue (UserInterface|CreateWidget "/Game/VFX_Chess/Assets/Cutscenes/Cutscene.Cutscene_C"))
  (UserInterface|Viewport|AddtoViewport _returnvalue 0)
  (Default|PlayCutscene _returnvalue _index))

(event EventBlackWin
  ;[1 1 1] Win conditions
  (bind _returnvalue (UserInterface|CreateWidget "/Game/VFX_Chess/Blueprints/UI/BlackVictory.BlackVictory_C"))
  (UserInterface|Viewport|AddtoViewport _returnvalue 0)
  (Input|SetInputModeUIOnly (Game|GetPlayerController 0) 0 "DoNotLock"))

(event EventWhiteWin
  ;[1 1 1] Win conditions
  (bind _returnvalue (UserInterface|CreateWidget "/Game/VFX_Chess/Blueprints/UI/WhiteVictory.WhiteVictory_C"))
  (UserInterface|Viewport|AddtoViewport _returnvalue 0)
  (Input|SetInputModeUIOnly (Game|GetPlayerController 0) 0 "DoNotLock"))

(event EventPlayCheckSound
  (Audio|PlaySound2D "/Game/VFX_Chess/Assets/Audio/Cues/check_Cue.check_Cue" 1.0 1.0 0.0 0 0))

(event EventPlayMovePieceSound
  (Audio|PlaySound2D "/Game/VFX_Chess/Assets/Audio/Cues/move_piece_Cue.move_piece_Cue" 1.0 1.0 0.0 0 0))

(event EventPlayPieceTaken
  (params (_pieceID :type Integer) (_isWhite :type Boolean))
  ;[1 1 1] Pieces taken
  (Audio|PlaySound2D "/Game/VFX_Chess/Assets/Audio/Cues/piece_taken_Cue.piece_taken_Cue" 1.0 1.0 0.0 0 0)
  (bind _foundwidgets (Widget|GetAllWidgetsOfClass "/Game/VFX_Chess/Blueprints/UI/PlayerHUD.PlayerHUD_C" true))
  (Default|OnPieceTaken (Utilities|Array|Get(acopy) _foundwidgets) _pieceID _isWhite))

(event EventPromotedPieceUI
  (params (_isWhite :type Boolean))
  ;[1 1 1] Pieces taken
  (if _isWhite
    (bind _returnvalue (UserInterface|CreateWidget "/Game/VFX_Chess/Blueprints/UI/PawnPromotionWhite.PawnPromotionWhite_C"))
    (UserInterface|Viewport|AddtoViewport _returnvalue 0)
    (else
      (bind _returnvalue_2 (UserInterface|CreateWidget "/Game/VFX_Chess/Blueprints/UI/PawnPromotionBlack.PawnPromotionBlack_C"))
      (UserInterface|Viewport|AddtoViewport _returnvalue_2 0)))
  (Input|SetInputModeUIOnly (Game|GetPlayerController 0) 0 "DoNotLock")
  (Variables|/Game/VFX_Chess/Blueprints/UI/PlayerHUD.PlayerHUD_C|SetWhitePromoted (Utilities|Array|Get(acopy) (stale EventPlayPieceTaken _foundwidgets)) _isWhite))

(event EventStalemate
  ;[1 1 1] Win conditions
  (bind _returnvalue (UserInterface|CreateWidget "/Game/VFX_Chess/Blueprints/UI/Stalemate.Stalemate_C"))
  (UserInterface|Viewport|AddtoViewport _returnvalue 0)
  (Input|SetInputModeUIOnly (Game|GetPlayerController 0) 0 "DoNotLock"))

(fn ConstructionScript)