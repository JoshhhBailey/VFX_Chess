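; BoneBreaker turns skeletal meshes into breakable physics objects, collapsing them wholly or from a hit point.
; BreakSkeleton branches on Modular: simulate physics from the parent of the hit bone downward, or from the bone at index zero.
; Both paths first apply the BreakProfile constraint profile to all joints, and the hit path can print its start bone for debugging.
; A separate DetachProp function releases a mesh in world space and enables physics on it.
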(event EventBeginPlay)

(event EventTick
  (params (DeltaSeconds :type Float%20%28single-precision%29)))

(fn BreakAll
  (params (Mesh :type Skeletal%20Mesh%20Component%20Object%20Reference))
  (Class|SkeletalMeshComponent|SetConstraintProfileforAll Mesh (Variables|BreakOptions|GetBreakProfile) true)
  (Class|SkeletalMeshComponent|SetAllBodiesBelowSimulatePhysics Mesh (Class|SkinnedMeshComponent|GetBoneName Mesh) true true))

(fn BreakClosestBone
  (params (Mesh :type Skeletal%20Mesh%20Component%20Object%20Reference) (HitResult :type Hit%20Result%20Structure))
  (bind _debughitbone (Variables|Debug|GetDebugHitBone))
  (bind _output_get (LocalVariables|SetSkelMesh Mesh))
  (LocalVariables|SetPhysicsStartBone (Class|SkinnedMeshComponent|GetParentBone (LocalVariables|GetSkelMesh) (.HitBoneName (Collision|BreakHitResult HitResult))))
  (Class|SkeletalMeshComponent|SetConstraintProfileforAll _output_get (Variables|BreakOptions|GetBreakProfile) false)
  (Development|PrintString (Utilities|String|ToString(Name) (Class|SkinnedMeshComponent|GetParentBone (LocalVariables|GetSkelMesh) (.HitBoneName (Collision|BreakHitResult HitResult)))) _debughitbone _debughitbone)
  ;[1 1 1] Simulate all bones below
  (Class|SkeletalMeshComponent|SetAllBodiesBelowSimulatePhysics (LocalVariables|GetSkelMesh) (LocalVariables|GetPhysicsStartBone) true true))

(fn DetachProp
  (params (Mesh :type Mesh%20Component%20Object%20Reference))
  (Transformation|DetachFromComponent Mesh "KeepWorld" "KeepWorld" "KeepWorld" true)
  (Physics|SetSimulatePhysics Mesh true))

(fn BreakSkeleton
  (params (Mesh :type Skeletal%20Mesh%20Component%20Object%20Reference) (HitResult :type Hit%20Result%20Structure))
  (LocalVariables|SetSkeletalMesh Mesh)
  (if (Variables|BreakOptions|GetModular)
    (CallFunction|BreakClosestBone (LocalVariables|GetSkeletalMesh) HitResult)
    (else
      (CallFunction|BreakAll (LocalVariables|GetSkeletalMesh)))))